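; BP_Panel is an interactable minigame panel that opens a linked door when its puzzle is completed.
; A box overlap tracks the nearby BP_MainCharacter as PlayerRef.
; Interacting blends the view to the panel's camera, hides the character mesh, disables its input and shows W_Minigame in UI-only input mode.
; The widget's OnPuzzleComplete dispatcher triggers the door and deactivates the panel, restoring the player's view, mesh and game input.
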(event OnComponentBeginOverlap(Box)
  (params (OverlappedComponent :type Primitive%20Component%20Object%20Reference) (OtherActor :type Actor%20Object%20Reference) (OtherComp :type Primitive%20Component%20Object%20Reference) (OtherBodyIndex :type Integer) (bFromSweep :type Boolean) (SweepResult :type Hit%20Result%20Structure%20%28by%20ref%29))
  ;[0.15 0.15 0.15 0.5] Setea el player cuando esta en rango del panel
  (bind _asbp_main_character (Utilities|Casting|CastToBP_MainCharacter OtherActor))
  (Variables|Default|SetPlayerRef _asbp_main_character))

(event OnComponentEndOverlap(Box)
  (params (OverlappedComponent :type Primitive%20Component%20Object%20Reference) (OtherActor :type Actor%20Object%20Reference) (OtherComp :type Primitive%20Component%20Object%20Reference) (OtherBodyIndex :type Integer))
  ;[0.15 0.15 0.15 0.5] Setea el player cuando esta en rango del panel
  (Utilities|Casting|CastToBP_MainCharacter OtherActor)
  (Variables|Default|SetPlayerRef 0))

(event Custom|ActivatePanel
  (bind _cameraref (Variables|Default|GetCameraRef))
  (Development|PrintString "Activating Panel")
  (Variables|Default|SetisActive true)
  (Variables|/Script/Engine.PlayerController|SetbShowMouseCursor (Variables|Default|GetPlayerController) true)
  (Input|DisableInput (Variables|Default|GetPlayerRef) (Variables|Default|GetPlayerController))
  (Development|PrintString (Utilities|String|Append "Camera is:" (Utilities|GetDisplayName _cameraref)))
  (Game|Player|SetViewTargetwithBlend (Variables|Default|GetPlayerController) _cameraref 1.0 "VTBlend_Cubic" 2.0 false)
  (bind _returnvalue (UserInterface|CreateWidget "/Game/Minigame/W_Minigame.W_Minigame_C" (Variables|Default|GetPlayerController)))
  (Variables|/Game/Minigame/W_Minigame.W_Minigame_C|SetBP_Panel _returnvalue self)
  (bind _output_get (Variables|Default|SetWidgetRef _returnvalue))
  (UserInterface|Viewport|AddtoViewport _output_get 0)
  (Input|SetInputModeUIOnly (Variables|Default|GetPlayerController) _output_get "DoNotLock" false)
  (EventDispatchers|AssignOnPuzzleComplete (Variables|Default|GetWidgetRef) (delegate Custom|OnPuzzleComplete_Event))
  (Rendering|SetVisibility (Variables|/Script/Engine.Character|GetMesh (Variables|Default|GetPlayerRef)) false false))

(event Custom|OnPuzzleComplete_Event
  (Default|OpenDoor (Variables|Default|GetDoorRef))
  (CallFunction|DeactivatePanel))

(event Custom|DeactivatePanel
  (Development|PrintString "Deactivating Panel")
  (Variables|Default|SetisActive false)
  (Game|Player|SetViewTargetwithBlend (Variables|Default|GetPlayerController) (Game|GetPlayerCharacter 0) 1.0 "VTBlend_Cubic" 2.0 false)
  (Rendering|SetVisibility (Variables|/Script/Engine.Character|GetMesh (Variables|Default|GetPlayerRef)) true true)
  (Input|SetInputModeGameOnly (Variables|Default|GetPlayerController) false)
  (Input|EnableInput (Variables|Default|GetPlayerRef) (Variables|Default|GetPlayerController))
  (if (Utilities|IsValid (Variables|Default|GetWidgetRef))
    (Widget|RemovefromParent (Variables|Default|GetWidgetRef))))

(event EventBeginPlay
  (bind _returnvalue (Class|InputDeviceLibrary|GetPlayerControllerfromInputDevice))
  (bind _output_get (Variables|Default|SetPlayerController _returnvalue))
  (Input|EnableInput _output_get))

(event Collision|EventActorBeginOverlap
  (params (OtherActor :type Actor%20Object%20Reference)))

(event EventTick
  (params (DeltaSeconds :type Float%20%28single-precision%29)))

(event EventInteract
  (params (player :type BP%20Main%20Character%20Object%20Reference))
  ;[0.15 0.15 0.15 0.5] Interact
  (CallFunction|ActivatePanel))

(fn ConstructionScript)

(fn NewFunction)