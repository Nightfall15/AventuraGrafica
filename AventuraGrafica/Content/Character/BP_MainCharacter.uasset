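; BP_MainCharacter is the player character, handling movement, mouse look, pausing and interaction.
; Axis inputs move it relative to control yaw, and Pause shows W_Pause with UI-only input and a paused game.
; Collision overlaps cache an IInteract component as DialogueActor or the actor as InteractActor, and any end overlap clears both.
; Interact sends InteractMessage to the cached component first, falling back to the actor.
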(event OnComponentBeginOverlap(Collision)
  (params (OverlappedComponent :type Primitive%20Component%20Object%20Reference) (OtherActor :type Actor%20Object%20Reference) (OtherComp :type Primitive%20Component%20Object%20Reference) (OtherBodyIndex :type Integer) (bFromSweep :type Boolean) (SweepResult :type Hit%20Result%20Structure%20%28by%20ref%29))
  ;[0.15 0.15 0.15 0.5] Player Interaction
  (Variables|Default|SetDialogueActor (Utilities|Array|Get(acopy) (Class|Actor|GetComponentsbyInterface OtherActor "/Game/DialogSystem/IInteract.IInteract_C")))
  (if (Utilities|DoesObjectImplementInterface OtherActor "/Game/DialogSystem/IInteract.IInteract_C")
    (Variables|Default|SetInteractActor OtherActor)))

(event OnComponentEndOverlap(Collision)
  (params (OverlappedComponent :type Primitive%20Component%20Object%20Reference) (OtherActor :type Actor%20Object%20Reference) (OtherComp :type Primitive%20Component%20Object%20Reference) (OtherBodyIndex :type Integer))
  ;[0.15 0.15 0.15 0.5] Player Interaction
  (Utilities|IsValid (Variables|Default|GetDialogueActor)
    (:Is%20Valid
      (Variables|Default|SetDialogueActor 0))
    (:Is%20Not%20Valid
      _))
  (Utilities|IsValid (Variables|Default|GetInteractActor)
    (:Is%20Valid
      (Variables|Default|SetInteractActor 0))))

(event Input|ActionEvents|InputActionPause
  (params (Key :type Key%20Structure :default "None"))
  (bind _returnvalue (Game|GetPlayerController 0))
  (:Pressed
    (bind _returnvalue_2 (UserInterface|CreateWidget "/Game/UI/PauseMenu/W_Pause.W_Pause_C"))
    (UserInterface|Viewport|AddtoViewport _returnvalue_2 0)
    (Variables|/Script/Engine.PlayerController|SetbShowMouseCursor _returnvalue true)
    (Input|SetInputModeUIOnly _returnvalue 0 "DoNotLock" false)
    (Game|SetGamePaused true)))

(event Input|ActionEvents|InputActionInteract
  (params (Key :type Key%20Structure :default "None"))
  (bind _self self)
  (bind _interactactor (Variables|Default|GetInteractActor))
  (bind _dialogueactor (Variables|Default|GetDialogueActor))
  ;[0.15 0.15 0.15 0.5] Player Interaction
  (:Pressed
    (Utilities|IsValid _dialogueactor
      (:Is%20Valid
        (Class|IInteract|Interact(Message) _dialogueactor _self))
      (:Is%20Not%20Valid
        (Utilities|IsValid _interactactor
          (:Is%20Valid
            (if (Utilities|DoesObjectImplementInterface _interactactor "/Game/DialogSystem/IInteract.IInteract_C")
              (Class|IInteract|Interact(Message) _interactactor _self))))))))

(event Input|AxisEvents|InputAxisGoRight/Left
  (params (AxisValue :type Float%20%28single-precision%29))
  ;[0.15 0.15 0.15 0.5] Movement
  (Pawn|Input|AddMovementInput (Math|Vector|GetRightVector (Math|Rotator|MakeRotator 0.0 0.0 (.yaw (Pawn|GetControlRotation :!class /Script/Engine.Pawn)))) AxisValue false))

(event Input|AxisEvents|InputAxisGoForward/Back
  (params (AxisValue :type Float%20%28single-precision%29))
  ;[0.15 0.15 0.15 0.5] Movement
  (Pawn|Input|AddMovementInput (Math|Vector|GetForwardVector (Math|Rotator|MakeRotator 0.0 0.0 (.yaw (Pawn|GetControlRotation :!class /Script/Engine.Pawn)))) AxisValue false))

(event Input|AxisEvents|InputAxisMouseUp/Down
  (params (AxisValue :type Float%20%28single-precision%29))
  ;[0.15 0.15 0.15 0.5] Camera
  (Pawn|Input|AddControllerPitchInput AxisValue))

(event Input|AxisEvents|InputAxisMouseRight/Left
  (params (AxisValue :type Float%20%28single-precision%29))
  ;[0.15 0.15 0.15 0.5] Camera
  (Pawn|Input|AddControllerYawInput AxisValue))

(fn ConstructionScript)